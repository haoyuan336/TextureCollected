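; Gun component for a tower defence tower that automatically aims and fires at tagged enemies within its yaw arc.
; Look and unlook events maintain a list of seen enemies, from which Tick locks a target inside the rotation limits and turns the gun toward it.
; A DoOnce-gated looping timer asks the owning TowerBaseCharacter_BP to fire by component index, and is cleared when the target is lost.
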(event Custom|LookActor
  (params (LookActor :type Actor%20Object%20Reference) (ComponentIndex :type Integer))
  (Variables|Default|SetComponentIndex ComponentIndex)
  (if (Actor|ActorHasTag LookActor (Variables|Default|GetTargetTag))
    (Utilities|Array|Add (Variables|Default|GetLookedEnemyList) LookActor)))

(event Custom|UnLookActor
  (params (UnLookActor :type Actor%20Object%20Reference))
  (if (Actor|ActorHasTag UnLookActor (Variables|Default|GetTargetTag))
    (for (_array_element _array_index) (Variables|Default|GetLookedEnemyList)
      (if (== _array_element UnLookActor)
        (Utilities|Array|RemoveIndex (Variables|Default|GetLookedEnemyList) _array_index)
        (if (== (Variables|Default|GetLockedEnemy) UnLookActor)
          (Variables|Default|SetLockedEnemy 0)
          (Utilities|Time|ClearandInvalidateTimerbyHandle (Variables|Default|GetShootBulletTimeHandler))
          (Utilities|FlowControl|DoOnce false) ; enters at Reset
        )))))

(event Custom|ShootOneBullet
  (bind _astower_base_character_bp (Utilities|Casting|CastToTowerBaseCharacter_BP (Components|GetOwner self)))
  (Default|ShootOneBullet _astower_base_character_bp (Variables|Default|GetComponentIndex)))

(event EventBeginPlay)

(event EventTick
  (params (DeltaSeconds :type Float%20%28single-precision%29))
  (if (Utilities|IsValid (Variables|Default|GetLockedEnemy))
    (bind _rotation (CallFunction|GetRotation (Variables|Default|GetLockedEnemy)))
    (Variables|Default|SetCurrentZRotation _rotation)
    (if (and (<= (Variables|Default|GetCurrentZRotation) (Variables|Default|GetMaxRatation)) (>= (Variables|Default|GetCurrentZRotation) (Variables|Default|GetMinRotation)))
      (Transformation|SetWorldRotation self (Math|Rotator|MakeRotator 0.0 0.0 (Variables|Default|GetCurrentZRotation)) false false)
      (Utilities|FlowControl|DoOnce false :!label _label
        (:Completed
          (bind _returnvalue (Utilities|Time|SetTimerbyFunctionName 0 "ShootOneBullet" 0.1 true))
          (Variables|Default|SetShootBulletTimeHandler _returnvalue)))
      (else
        (Variables|Default|SetLockedEnemy 0)
        (Utilities|Time|ClearandInvalidateTimerbyHandle (Variables|Default|GetShootBulletTimeHandler))
        (goto _label Reset)))
    (else
      (bind _lockactor (CallFunction|FindCanAttackEnemy))
      (Variables|Default|SetLockedEnemy _lockactor))))

(fn GetRotation
  (params (TargetActor :type Actor%20Object%20Reference))
  (return (+ (.yaw (Math|Rotator|MakeRotfromZ (- (- (Transformation|GetActorLocation TargetActor) (Transformation|GetActorLocation (Components|GetOwner self))) (Transformation|GetActorForwardVector (Components|GetOwner self))))) -9e+01)))

(fn CheckCanAttack
  (params (LockedActor :type Actor%20Object%20Reference))
  (bind _rotation (CallFunction|GetRotation LockedActor))
  (return (and (<= _rotation (Variables|Default|GetMaxRatation)) (>= _rotation (Variables|Default|GetMinRotation)))))

(fn FindCanAttackEnemy
  (for _array_element (Variables|Default|GetLookedEnemyList)
    (bind _rotation (CallFunction|GetRotation _array_element))
    (if (and (<= _rotation (Variables|Default|GetMaxRatation)) (>= _rotation (Variables|Default|GetMinRotation)))
      (Variables|Default|SetLockedEnemy _array_element)))
  (return (Variables|Default|GetLockedEnemy)))