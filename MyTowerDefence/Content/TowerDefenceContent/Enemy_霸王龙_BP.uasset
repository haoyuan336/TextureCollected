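; Tyrannosaurus (霸王龙) enemy Blueprint for the tower defence game, a child class that supplies this dinosaur's attack animation.
; 播放攻击动画 casts the mesh's anim instance to 霸王龙_Anim_BP, triggers its attack and binds to its AttackPlayerEnd dispatcher.
; When that fires, it calls 攻击动画播放结束, which is defined outside this graph, to signal the attack has finished.
; BeginPlay, overlap and Tick are disabled stubs.
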(event Custom|攻击动画播放over
  (CallFunction|攻击动画播放结束))

(event EventBeginPlay
  (|CallParentFunction) ; 此节点被禁用，将不会被调用。\n从引脚连出引线来编译功能。
)

(event Collision|EventActorBeginOverlap
  (params (OtherActor :type Actor%20Object%20Reference))
  (|CallParentFunction OtherActor) ; 此节点被禁用，将不会被调用。\n从引脚连出引线来编译功能。
)

(event EventTick
  (params (DeltaSeconds :type Float%20%28single-precision%29))
  (|CallParentFunction DeltaSeconds) ; 此节点被禁用，将不会被调用。\n从引脚连出引线来编译功能。
)

(event Event播放攻击动画
  (bind _as霸王龙_anim_bp (Utilities|Casting|CastTo霸王龙_Anim_BP (Components|SkeletalMesh|GetAnimInstance (Variables|Character|GetMesh))))
  (Default|攻击 _as霸王龙_anim_bp)
  (EventDispatchers|BindEventtoAttackPlayerEnd _as霸王龙_anim_bp (delegate Custom|攻击动画播放over)))

(fn ConstructionScript
  (|CallParentFunction))