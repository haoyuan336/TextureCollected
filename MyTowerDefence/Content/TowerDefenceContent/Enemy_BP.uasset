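; Enemy character Blueprint for a tower defence game, serving as the pawn driven by Enemy_AI_Controller.
; When MoveToEnemyCollision overlaps an actor tagged Player, it tells the AI controller it has moved close to its enemy.
; A ChangeSpeed event sets max walk speed, and the attack-animation-end event fires a finished dispatcher.
; The play-attack-animation event and mesh overlap handler are empty here.
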(event OnComponentBeginOverlap(Mesh)
  (params (OverlappedComponent :type Primitive%20Component%20Object%20Reference) (OtherActor :type Actor%20Object%20Reference) (OtherComp :type Primitive%20Component%20Object%20Reference) (OtherBodyIndex :type Integer) (bFromSweep :type Boolean) (SweepResult :type Hit%20Result%20Structure%20%28by%20ref%29)))

(event OnComponentBeginOverlap(MoveToEnemyCollision)
  (params (OverlappedComponent :type Primitive%20Component%20Object%20Reference) (OtherActor :type Actor%20Object%20Reference) (OtherComp :type Primitive%20Component%20Object%20Reference) (OtherBodyIndex :type Integer) (bFromSweep :type Boolean) (SweepResult :type Hit%20Result%20Structure%20%28by%20ref%29))
  (if (Actor|ActorHasTag OtherActor "Player")
    (bind _asenemy_ai_controller (Utilities|Casting|CastToEnemy_AI_Controller (AI|GetAIController self)))
    (Default|MovedCloseEnemy _asenemy_ai_controller)))

(event Custom|ChangeSpeed
  (params (Speed :type Float%20%28single-precision%29))
  (Variables|/Script/Engine.CharacterMovementComponent|SetMaxWalkSpeed (Variables|Character|GetCharacterMovement) Speed))

(event Custom|播放攻击动画)

(event Custom|攻击动画播放结束
  (Default|Call攻击动画播放完毕))

(event EventBeginPlay)

(event Collision|EventActorBeginOverlap
  (params (OtherActor :type Actor%20Object%20Reference)))

(event EventTick
  (params (DeltaSeconds :type Float%20%28single-precision%29)))

(fn ConstructionScript)